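; Player character with axis movement, jump, crouch and adjustable camera sensitivity and Y inversion, plus a pausing settings menu on key 1.
; FOV and capsule overlaps set seen and in-room flags on BP_DisappearingItem, replacing a disconnected line trace.
; Sphere overlap with a keycard increments the key count and shows a timed prompt.
; E collects the card or decrements the count, but door handling is unfinished.
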(event `InputAxis|ForwardBack`
  (params (AxisValue :type "Float (single-precision)"))
  ;[1 1 1] WASD Movement (Ace)
  (`self.AddMovementInput` (`self.GetActorForwardVector`) (* (`self.MaxSpeed`) AxisValue)))

(event `Key|SpaceBar`
  (params (Key :type "Key Structure"))
  ;[1 1 1] Jump (Ace)
  (:`Pressed`
    (`self.Jump`)))

(event `InputAxis|LeftRight`
  (params (AxisValue :type "Float (single-precision)"))
  ;[1 1 1] WASD Movement (Ace)
  (`self.AddMovementInput` (`self.GetActorRightVector`) (* (`self.MaxSpeed`) AxisValue)))

(event `Key|K`
  (params (Key :type "Key Structure"))
  ;[1 1 1] Alternate between Gravity on and gravity off speed (gravity not included lol) (Ace)
)

(event `InputAxis|CameraX`
  (params (AxisValue :type "Float (single-precision)"))
  ;[1 1 1] Camera (Ace)
  (`self.AddControllerYawInput` (* AxisValue (`self.CamXSensitivity`))))

(event `Key|LeftControl`
  (params (Key :type "Key Structure"))
  ;[1 1 1] Crouch (Ace)
  (:`Pressed`
    (`self.Crouch`))
  (:`Released`
    (`self.UnCrouch`)))

(event `InputAxis|CameraY`
  (params (AxisValue :type "Float (single-precision)"))
  ;[1 1 1] Camera (Ace)
  (`self.AddControllerPitchInput` (* AxisValue (`self.CamYInvertVal`) (`self.CamYSensitivity`))))

(event `Key|One` :paused true
  (params (Key :type "Key Structure"))
  (bind _returnvalue (`GameplayStatics.GetPlayerController` 0))
  (bind _returnvalue_2 (`GameplayStatics.GetPlayerController` 0))
  ;[1 1 1] Sensitivity Slider widgets menu, to be implemented into final settings menu. Also CamYInvert at the end (Ace)
  (:`Pressed`
    (if (`GameplayStatics.IsGamePaused`)
      (`GameplayStatics.SetGamePaused` false)
      (`Widget.RemoveFromParent` (stale _returnvalue_3))
      (`WidgetBlueprintLibrary.SetInputMode_GameOnly` _returnvalue)
      (set `PlayerController.bShowMouseCursor` false _returnvalue)
      (`self.SetYInvert`)
      (else
        (`GameplayStatics.SetGamePaused` true)
        (bind _returnvalue_3 (`|CreateWidget` "/Game/Widgets/BP_AceMenu.BP_AceMenu_C"))
        (`UserWidget.AddToViewport` _returnvalue_3 0)
        (`WidgetBlueprintLibrary.SetInputMode_GameAndUIEx` _returnvalue_2 null "DoNotLock" false)
        (set `PlayerController.bShowMouseCursor` true _returnvalue_2)
        (`self.SetYInvert`)))))

(event `self.FOV.OnComponentBeginOverlap`
  (params (OverlappedComponent :type "PrimitiveComponent Object Reference") (OtherActor :type "Actor Object Reference") (OtherComp :type "PrimitiveComponent Object Reference") (OtherBodyIndex :type Integer) (bFromSweep :type Boolean) (SweepResult :type "HitResult Structure (by ref)"))
  ;[0.2753 1 0.5184] Component Overlap BP_DissappearingItem w/ FOV (MARK)
  (bind _asbp_disappearing_item (cast `/Game/Blueprints/BP_DisappearingItem` OtherActor))
  (set `/Game/Blueprints/BP_DisappearingItem.IsNotVisible` false _asbp_disappearing_item)
  (set `/Game/Blueprints/BP_DisappearingItem.LookedAt` true _asbp_disappearing_item))

(event `self.FOV.OnComponentEndOverlap`
  (params (OverlappedComponent :type "PrimitiveComponent Object Reference") (OtherActor :type "Actor Object Reference") (OtherComp :type "PrimitiveComponent Object Reference") (OtherBodyIndex :type Integer))
  ;[0.2753 1 0.5184] Component Overlap BP_DissappearingItem w/ FOV (MARK)
  (bind _asbp_disappearing_item (cast `/Game/Blueprints/BP_DisappearingItem` OtherActor))
  (set `/Game/Blueprints/BP_DisappearingItem.IsNotVisible` true _asbp_disappearing_item))

(event `self.CapsuleComponent.OnComponentBeginOverlap`
  (params (OverlappedComponent :type "PrimitiveComponent Object Reference") (OtherActor :type "Actor Object Reference") (OtherComp :type "PrimitiveComponent Object Reference") (OtherBodyIndex :type Integer) (bFromSweep :type Boolean) (SweepResult :type "HitResult Structure (by ref)"))
  ;[0.2753 1 0.5184] Component Overlap BP_DissappearingItem w/ FOV (MARK)
  (bind _asbp_disappearing_item (cast `/Game/Blueprints/BP_DisappearingItem` OtherActor))
  (set `/Game/Blueprints/BP_DisappearingItem.InTheRoom` true _asbp_disappearing_item))

(event `self.CapsuleComponent.OnComponentEndOverlap`
  (params (OverlappedComponent :type "PrimitiveComponent Object Reference") (OtherActor :type "Actor Object Reference") (OtherComp :type "PrimitiveComponent Object Reference") (OtherBodyIndex :type Integer))
  ;[0.2753 1 0.5184] Component Overlap BP_DissappearingItem w/ FOV (MARK)
  (bind _asbp_disappearing_item (cast `/Game/Blueprints/BP_DisappearingItem` OtherActor))
  (set `/Game/Blueprints/BP_DisappearingItem.InTheRoom` false _asbp_disappearing_item))

(event `self.Sphere Collision.OnComponentBeginOverlap`
  (params (OverlappedComponent :type "PrimitiveComponent Object Reference") (OtherActor :type "Actor Object Reference") (OtherComp :type "PrimitiveComponent Object Reference") (OtherBodyIndex :type Integer) (bFromSweep :type Boolean) (SweepResult :type "HitResult Structure (by ref)"))
  ;[0.8549 0.3125 1] Keycard and Door (Sam)
  (bind _asbp_key_card (cast `/Game/Blueprints/BP_KeyCard` OtherActor)
    (:`then`
      (set `self.CanPickUp` true)
      (`Widget.RemoveFromParent` (`self.Interaction`))
      (set `self.As BP Key Card` _asbp_key_card)
      (`/Engine/EditorBlueprintResources/StandardMacros.IncrementInt` (`self.keycount`)
        (:`  `
          (bind _returnvalue (`|CreateWidget` "/Game/Widgets/WB_Interaction.WB_Interaction_C"))
          (bind _output_get (set `self.Interaction` _returnvalue))
          (`UserWidget.AddToViewport` _output_get 0)
          (`KismetSystemLibrary.Delay` 3.0)
          (`WidgetLayoutLibrary.RemoveAllWidgets`))))
    (:`CastFailed`
      (cast `/Game/Blueprints/Interactions/BP_Door` OtherActor)
      (if (> (`self.keycount`) 0)
        _))))

(event `Key|E`
  (params (Key :type "Key Structure"))
  (bind _as_bp_door (`self.As BP Door`))
  ;[0.8549 0.3125 1] Keycard and Door (Sam)
  (:`Pressed`
    (if (`self.CanPickUp`)
      (`self.K2_DestroyActor` (`self.As BP Key Card`))
      (set `self.HasKey?` true)
      (else
        (`/Engine/EditorBlueprintResources/StandardMacros.IsValid` _as_bp_door ; Is there a door close?
          (:`Is Valid`
            (`/Engine/EditorBlueprintResources/StandardMacros.DecrementInt` (`self.keycount`) ; Subtract 1 key
              (:`  `
                (cast `/Game/Blueprints/Interactions/BP_Door` _as_bp_door)))))))))

(fn `SetYInvert`
  (if (`self.CamYInvert`)
    (set `self.CamYInvertVal` -1)
    (else
      (set `self.CamYInvertVal` 1))))

(fn `UserConstructionScript`)