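; BP_DisappearingItem is an actor that removes itself once the player has seen it and it is out of view while the player is in the room.
; Each tick it destroys itself when the IsNotVisible, LookedAt and InTheRoom flags are all true.
; No live graph sets those flags to true; leftover overlap-binding and teleport nodes are marked obsolete or never run.
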(event `self.ReceiveTick`
  (params (DeltaSeconds :type "Float (single-precision)"))
  ;[0.05566 0.8076 1] Every tick, if the varibles IsNotVisible and LookedAt are true and the player character is in the room trigger, the item is deleted.
  (if (`self.IsNotVisible`)
    (if (`self.LookedAt`)
      (if (`self.InTheRoom`)
        (`self.K2_DestroyActor`)))))

(event `OnActorEndOverlap_Event` :!signature `self.OnActorEndOverlap`
  (params (OverlappedActor :type "Actor Object Reference") (OtherActor :type "Actor Object Reference"))
  ;[0.1885 0.1885 0.1885] OLD DON'T NEED
  (add `self.OnActorEndOverlap` OverlappedActor (delegate `OnActorEndOverlap_Event`))
  (set `self.IsNotVisible` false))

(fn `UserConstructionScript`)