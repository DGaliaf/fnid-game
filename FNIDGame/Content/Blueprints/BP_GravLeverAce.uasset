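; BP_GravLeverAce is an interactable lever that switches on the gravity areas in the level.
; On InteractwithObject it gathers every BP_GravAreaAce actor and sets SwitchFlipped on each, looping by an ArrayNum index that is never reset.
; When the index finds no valid actor, it prints a debug "Hello" and plays the FlipLever timeline, which rolls the Lever component to its flipped position.
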(event `self.InteractWithObject`
  (bind _outactors (`GameplayStatics.GetAllActorsOfClass` "/Game/Blueprints/BP_GravAreaAce.BP_GravAreaAce_C" :!label _label))
  (bind _output (`|GetArrayItem` _outactors (`self.ArrayNum`)))
  (`/Engine/EditorBlueprintResources/StandardMacros.IsValid` _output
    (:`Is Valid`
      (set `/Game/Blueprints/BP_GravAreaAce.SwitchFlipped` true _output)
      (`/Engine/EditorBlueprintResources/StandardMacros.IncrementInt` (`self.ArrayNum`)
        (:`  `
          (goto _label))))
    (:`Is Not Valid`
      (`KismetSystemLibrary.PrintString` "Hello")
      (bind (_direction _newtrack_0) (`Timeline|Flip lever`)
        (:`Update`
          (`SceneComponent.K2_SetRelativeRotation` (`self.Lever`) (`KismetMathLibrary.MakeRotator` (`KismetMathLibrary.Lerp` 50.0 130.0 _newtrack_0)) false false))))))

(fn `UserConstructionScript`
  (`parent.UserConstructionScript`))