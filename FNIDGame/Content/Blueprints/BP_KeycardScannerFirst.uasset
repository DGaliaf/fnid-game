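; Keycard scanner Blueprint that gates a sliding double door behind the player's keycard.
; On interaction it checks keycard and door-check flags in the game instance, playing a fail sequence without a card.
; With a card, an unset DoorCheck plays the pass sequence and reveals the correct ID card mesh.
; A set DoorCheck plays the open sequence on a closed door while a Timeline slides both panels apart and marks it open.
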(event `self.InteractWithObject`
  (`SequenceEvaluatorLibrary.SetSequence` (`self.IdScanSuccess`) "/Game/Animations/RightID/IDScanSuccess_ANI_Anim.IDScanSuccess_ANI_Anim")
  (bind _asbp_door (cast `/Game/Blueprints/Interactions/BP_Door` (`self.OtherActor`)))
  ;[1 1 1] Check if Door Can be Opened
  (bind _asbp_game_variables (cast `/Game/Blueprints/BP_GameVariables` (`GameplayStatics.GetGameInstance`)))
  (if (`/Game/Blueprints/BP_GameVariables.KeyCardObtained` _asbp_game_variables)
    (if (not (`/Game/Blueprints/BP_GameVariables.DoorCheck` _asbp_game_variables))
      (`MovieSceneSequencePlayer.Play` (`LevelSequenceActor.SequencePlayer` (`self.Level Sequence Pass`)))
      (bind _asbp_correct_id (cast `/Game/Blueprints/Interactions/BP_CorrectID` (`self.ID Card`)))
      (`SceneComponent.SetVisibility` (`/Game/Blueprints/Interactions/BP_CorrectID.Cube` _asbp_correct_id) true false)
      (elif (not (`/Game/Blueprints/Interactions/BP_Door.DoorOpen` _asbp_door))
        (`MovieSceneSequencePlayer.Play` (`LevelSequenceActor.SequencePlayer` (`self.Level Sequence Open`)))
        (bind (_direction _newtrack_0) (`Timeline|Timeline` :!via `PlayFromStart`)
          (:`Update`
            (bind _doorr (`/Game/Blueprints/Interactions/BP_Door.DoorR` _asbp_door))
            (bind (_relativelocation_x _relativelocation_y _relativelocation_z) (`KismetMathLibrary.BreakVector` (`SceneComponent.RelativeLocation` _doorr)))
            (`SceneComponent.K2_SetRelativeLocation` _doorr (`KismetMathLibrary.MakeVector` (* _newtrack_0 190.0) _relativelocation_y _relativelocation_z) false false)
            (bind _doorl (`/Game/Blueprints/Interactions/BP_Door.DoorL` _asbp_door))
            (bind (_relativelocation_x_2 _relativelocation_y_2 _relativelocation_z_2) (`KismetMathLibrary.BreakVector` (`SceneComponent.RelativeLocation` _doorl)))
            (`SceneComponent.K2_SetRelativeLocation` _doorl (`KismetMathLibrary.MakeVector` (* _newtrack_0 -190.0) _relativelocation_y_2 _relativelocation_z_2) false false)
            (set `/Game/Blueprints/Interactions/BP_Door.DoorOpen` true _asbp_door)))))
    (else
      (`MovieSceneSequencePlayer.Play` (`LevelSequenceActor.SequencePlayer` (`self.Level Sequence Fail`))))))

(fn `UserConstructionScript`
  (`parent.UserConstructionScript`))