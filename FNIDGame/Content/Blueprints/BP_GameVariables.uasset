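; Holds shared game progress state and handles saving and loading of the player's position.
; Init resets the puzzle flags for circuit, buttons and key card, the bedroom object count, and temporary wire endpoints.
; Load reads or creates a BP_SaveGame, then teleports the player pawn to its stored transform, even for a new save.
; Save writes only the pawn's transform to a single slot, leaving progress unsaved.
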(event `self.ReceiveInit`
  (set `self.CircuitComplete` false)
  (set `self.ButtonsCompelte` false)
  (set `self.KeyCardObtained` false)
  (set `self.BedroomObjectsCollected` 0)
  (set `self.TempStartWire` -1)
  (set `self.TempEndWire` -1))

(event `Load`
  (bind _returnvalue (`GameplayStatics.DoesSaveGameExist` "save1"))
  (if _returnvalue
    (bind _returnvalue_2 (`GameplayStatics.LoadGameFromSlot` "save1"))
    (bind _asbp_save_game (cast `/Game/Blueprints/SaveSystem/BP_SaveGame` _returnvalue_2))
    (set `self.As BP Save Game` _asbp_save_game)
    (else
      (bind _returnvalue_3 (`GameplayStatics.CreateSaveGameObject` "/Game/Blueprints/SaveSystem/BP_SaveGame.BP_SaveGame_C"))
      (set `self.As BP Save Game` _returnvalue_3)))
  (`Actor.K2_SetActorTransform` (`GameplayStatics.GetPlayerPawn` 0) (`/Game/Blueprints/SaveSystem/BP_SaveGame.PlayerPos` (`self.As BP Save Game`)) false false))

(event `Save`
  (bind _as_bp_save_game (`self.As BP Save Game`))
  (`/Engine/EditorBlueprintResources/StandardMacros.IsValid` _as_bp_save_game
    (:`Is Valid`
      _)
    (:`Is Not Valid`
      (bind _returnvalue (`GameplayStatics.CreateSaveGameObject` "/Game/Blueprints/SaveSystem/BP_SaveGame.BP_SaveGame_C"))
      (set `self.As BP Save Game` _returnvalue)))
  (set `/Game/Blueprints/SaveSystem/BP_SaveGame.PlayerPos` (`Actor.GetTransform` (`GameplayStatics.GetPlayerPawn` 0)) _as_bp_save_game)
  (`GameplayStatics.SaveGameToSlot` (`self.As BP Save Game`) "Save1"))