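; Player character Blueprint that handles movement, camera, jumping, the crosshair, a tabbed menu and a pause menu.
; BeginPlay creates the widgets, input opens them with game pause and input-mode switches, and the IsMenuClosed macro gates movement while a Processing flag guards menu toggles.
; AddItem and SwapItem link BPCInventory to the menu.
; Debug keys start quests, add a test item and toggle forward speed; the crosshair interaction trace is disconnected.
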(event `ResumePressed`
  (bind _returnvalue (`GameplayStatics.GetPlayerController` 0))
  (bind _pausemenu (`self.PauseMenu`))
  ;[1 0.3968 0.7011] Open Pause Menu (Keagon)
  (`KismetSystemLibrary.PrintString` "CharacterResumePressed")
  (if (`self.PauseOpen`) :!label _label
    (set `self.PauseOpen` false)
    (`Widget.RemoveFromParent` _pausemenu)
    (if (not (`self.MenuOpen`))
      (`GameplayStatics.SetGamePaused` false)
      (`WidgetBlueprintLibrary.SetInputMode_GameOnly` _returnvalue)
      (set `PlayerController.bShowMouseCursor` false _returnvalue)
      (else
        (set `PlayerController.bShowMouseCursor` true _returnvalue :!label _label_2)))
    (else
      (set `self.PauseOpen` true)
      (`UserWidget.AddToViewport` _pausemenu 0)
      (`GameplayStatics.SetGamePaused` true)
      (`WidgetBlueprintLibrary.SetInputMode_GameAndUIEx` _returnvalue _pausemenu "DoNotLock" false)
      (goto _label_2))))

(event `self.ReceiveTick`
  (params (DeltaSeconds :type "Float (single-precision)"))
  ;[1 0.3961 0.702] Crosshair detection (Keagon)
)

(event `EnhancedInput|/Game/Inputs/InputMaps/IA_OpenPause`
  (params (ActionValue :type Boolean) (ElapsedSeconds :type "Float (double-precision)") (TriggeredSeconds :type "Float (double-precision)") (InputAction :type "InputAction Object Reference" :default "/Game/Inputs/InputMaps/IA_OpenPause.IA_OpenPause"))
  ;[1 0.3968 0.7011] Open Pause Menu (Keagon)
  (:`Started`
    (if (`self.Processing`) :!label _label_3
      (`KismetSystemLibrary.Delay` 0.5)
      (goto _label_3)
      (elif (`self.SaveDisabled`)
        (`KismetSystemLibrary.PrintText` "Save Disabled")
        (goto _label)
        (else
          (goto _label))))))

(event `EnhancedInput|/Game/Inputs/InputMaps/IA_OpenMenu`
  (params (ActionValue :type Boolean) (ElapsedSeconds :type "Float (double-precision)") (TriggeredSeconds :type "Float (double-precision)") (InputAction :type "InputAction Object Reference" :default "/Game/Inputs/InputMaps/IA_OpenMenu.IA_OpenMenu"))
  (bind _returnvalue (`GameplayStatics.GetPlayerController` 0))
  (bind _menu (`self.Menu`))
  (bind (_sizex _sizey) (`PlayerController.GetViewportSize` _returnvalue))
  ;[1 0.3968 0.7011] Opening Menu (Keagon)
  (:`Started`
    (`/Game/Widgets/WP_Menu.Tasks` (`self.Menu`))
    (if (not (`self.Processing`)) :!label _label_4
      (set `self.Processing` true)
      (if (`self.MenuOpen`)
        (set `PlayerController.bShowMouseCursor` false _returnvalue)
        (`WidgetBlueprintLibrary.SetInputMode_GameOnly` _returnvalue)
        (`Widget.SetVisibility` _menu "Hidden")
        (`GameplayStatics.SetGamePaused` false)
        (`KismetSystemLibrary.Delay` (`self.CloseDelay`))
        (set `self.MenuOpen` false)
        (set `self.Processing` false)
        (`Image.SetOpacity` (`/Game/Widgets/W_Crosshair.Crosshair_Dot` (`self.Crosshair`)) 0.75)
        (`Widget.SetIsEnabled` (`/Game/Widgets/WP_Menu.Button_Tasks` (`self.Menu`)) true)
        (`Widget.SetIsEnabled` (`/Game/Widgets/WP_Menu.Button_Logs` (`self.Menu`)) true)
        (`Widget.SetIsEnabled` (`/Game/Widgets/WP_Menu.Button_Data` (`self.Menu`)) true)
        (else
          (`Image.SetOpacity` (`/Game/Widgets/W_Crosshair.Crosshair_Dot` (`self.Crosshair`)) 0.0)
          (set `self.MenuOpen` true)
          (`KismetSystemLibrary.Delay` (`self.OpenDelay`))
          (`GameplayStatics.SetGamePaused` true)
          (`WidgetSwitcher.SetActiveWidgetIndex` (`/Game/Widgets/WP_Menu.WidgetSwitcher` _menu) (`self.WidgetID`))
          (`Widget.SetVisibility` _menu "Visible")
          (set `PlayerController.bShowMouseCursor` true _returnvalue)
          (`PlayerController.SetMouseLocation` _returnvalue (/ _sizex 2) (/ _sizey 2))
          (`WidgetBlueprintLibrary.SetInputMode_GameAndUIEx` _returnvalue _menu)
          (set `self.Processing` false))))))

(event `EnhancedInput|/Game/Inputs/InputMaps/IA_OpenMap`
  (params (ActionValue :type Boolean) (ElapsedSeconds :type "Float (double-precision)") (TriggeredSeconds :type "Float (double-precision)") (InputAction :type "InputAction Object Reference" :default "/Game/Inputs/InputMaps/IA_OpenMap.IA_OpenMap"))
  ;[1 0.3968 0.7011] Opening Menu (Keagon)
  (:`Started`
    (`/Game/Widgets/WP_Menu.Logs` (`self.Menu`))
    (goto _label_4)))

(event `EnhancedInput|/Game/Inputs/InputMaps/IA_OpenSettings`
  (params (ActionValue :type Boolean) (ElapsedSeconds :type "Float (double-precision)") (TriggeredSeconds :type "Float (double-precision)") (InputAction :type "InputAction Object Reference" :default "/Game/Inputs/InputMaps/IA_OpenSettings.IA_OpenSettings"))
  ;[1 0.3968 0.7011] Opening Menu (Keagon)
  (:`Started`
    (`/Game/Widgets/WP_Menu.Data` (`self.Menu`))
    (goto _label_4)))

(event `Key|K`
  (params (Key :type "Key Structure"))
  ;[1 1 1] Alternate between Gravity on and gravity off speed (gravity not included lol) (Ace)
  (:`Pressed`
    (`/Engine/EditorBlueprintResources/StandardMacros.FlipFlop`
      (:`A`
        (set `self.MaxSpeed` 0.2))
      (:`B`
        (set `self.MaxSpeed` 1.0)))))

(event `InputAxis|ForwardBack`
  (params (AxisValue :type "Float (single-precision)"))
  ;[1 1 1] WASD Movement (Ace)
  (`self.IsMenuClosed`
    (:`then`
      (`self.AddMovementInput` (`self.GetActorForwardVector`) (* (`self.MaxSpeed`) AxisValue)))))

(event `Key|SpaceBar`
  (params (Key :type "Key Structure"))
  ;[1 1 1] Jump (Ace)
  (:`Pressed`
    (`self.IsMenuClosed`
      (:`then`
        (`self.Jump`)))))

(event `InputAxis|LeftRight`
  (params (AxisValue :type "Float (single-precision)"))
  ;[1 1 1] WASD Movement (Ace)
  (`self.IsMenuClosed`
    (:`then`
      (`self.AddMovementInput` (`self.GetActorRightVector`) AxisValue))))

(event `InputAxis|CameraX`
  (params (AxisValue :type "Float (single-precision)"))
  ;[1 1 1] Camera (Ace)
  (`self.IsMenuClosed`
    (:`then`
      (`self.AddControllerYawInput` (* AxisValue (`self.CamXSensitivity`))))))

(event `InputAxis|CameraY`
  (params (AxisValue :type "Float (single-precision)"))
  ;[1 1 1] Camera (Ace)
  (`self.IsMenuClosed`
    (:`then`
      (`self.AddControllerPitchInput` (* AxisValue (`self.CamYInvertVal`) (`self.CamYSensitivity`))))))

(event `Key|Eight`
  (params (Key :type "Key Structure")))

(event `self.ReceiveBeginPlay`
  (bind _returnvalue (`GameplayStatics.GetPlayerController` 0))
  (bind _menu (`self.Menu`))
  (bind _returnvalue_2 (pcsubsystem `EnhancedInputLocalPlayerSubsystem` _returnvalue))
  ;[1 1 1] CamYInvert (Ace)
  (`|ExecutionSequence`
    (:`then_0`
      (if (`self.CamYInvert`)
        (set `self.CamYInvertVal` -1)
        (else
          (set `self.CamYInvertVal` 1))))
    (:`then_1`
      ;[1 0.3968 0.7011] Menu Setup (Keagon)
      (bind _returnvalue_3 (`|CreateWidget` "/Game/Widgets/W_Crosshair.W_Crosshair_C"))
      (bind _output_get (set `self.Crosshair` _returnvalue_3))
      (`UserWidget.AddToViewport` _output_get 0)
      (`/Engine/EditorBlueprintResources/StandardMacros.IsValid` _returnvalue_2
        (:`Is Valid`
          (`EnhancedInputSubsystemInterface.AddMappingContext` _returnvalue_2 "/Game/Inputs/IMC_Basic.IMC_Basic" 0 (struct))
          (bind _returnvalue_4 (`|CreateWidget` "/Game/Widgets/WP_Menu.WP_Menu_C"))
          (set `self.Menu` _returnvalue_4)
          (`self.EnableInput` _returnvalue)
          (set `self.OpenDelay` 0.0)
          (set `self.MenuOpen` false)
          (set `self.CloseDelay` 0.0)
          (`Image.SetOpacity` (`/Game/Widgets/W_Crosshair.Crosshair_Dot` (`self.Crosshair`)) 0.0))))
    (:`then_2`
      (bind _returnvalue_5 (`|CreateWidget` "/Game/Widgets/WP_Tasks.WP_Tasks_C"))
      (set `self.TasksMenu` _returnvalue_5)
      (bind _returnvalue_6 (`|CreateWidget` "/Game/Widgets/WP_Log.WP_Log_C"))
      (set `self.LogMenu` _returnvalue_6)
      (bind _returnvalue_7 (`|CreateWidget` "/Game/Widgets/WP_Data.WP_Data_C"))
      (set `self.DataMenu` _returnvalue_7)
      (bind _returnvalue_8 (`|CreateWidget` "/Game/Widgets/W_PauseMenu.W_PauseMenu_C"))
      (set `self.PauseMenu` _returnvalue_8)
      (`UserWidget.AddToViewport` _menu 0)
      (`Widget.SetVisibility` _menu "Hidden"))))

(event `Key|Nine`
  (params (Key :type "Key Structure"))
  (:`Pressed`
    (bind _output_get (set `self.TestText` "TESTTESTTESTTESTTEST"))
    (`self.AddItem` _output_get _output_get (`self.Item Image`))))

(event `Key|Q`
  (params (Key :type "Key Structure"))
  (:`Pressed`
    (set `/Game/Widgets/WP_Menu.QuestIndex` 1 (`self.Menu`))
    (`/Game/Widgets/WP_Menu.StartQuest` (`self.Menu`) :!label _label_5)))

(event `Key|Two`
  (params (Key :type "Key Structure"))
  ;[1 1 1] Ace WIP Sensitivity Slider widgets (you may ignore) (Ace)
)

(event `Key|J`
  (params (Key :type "Key Structure"))
  (:`Pressed`
    (set `/Game/Widgets/WP_Menu.SubQuest1Complete` false (`self.Menu`))))

(event `Key|Two`
  (params (Key :type "Key Structure"))
  (:`Pressed`
    (set `/Game/Widgets/WP_Menu.QuestIndex` 2 (`self.Menu`))
    (goto _label_5)))

(event `Key|Three`
  (params (Key :type "Key Structure"))
  (:`Pressed`
    (set `/Game/Widgets/WP_Menu.QuestIndex` 3 (`self.Menu`))
    (goto _label_5)))

(event `Key|Four`
  (params (Key :type "Key Structure"))
  (:`Pressed`
    (set `/Game/Widgets/WP_Menu.QuestIndex` 4 (`self.Menu`))
    (goto _label_5)))

(event `Key|Five`
  (params (Key :type "Key Structure"))
  (:`Pressed`
    (set `/Game/Widgets/WP_Menu.QuestIndex` 5 (`self.Menu`))
    (goto _label_5)))

(event `Gameplay Start`
  ;[1 0.3968 0.7011] Set Crosshair Visible (Keagon)
  (`Image.SetOpacity` (`/Game/Widgets/W_Crosshair.Crosshair_Dot` (`self.Crosshair`)) 0.75))

(event `Key|Six`
  (params (Key :type "Key Structure"))
  (:`Pressed`
    (set `/Game/Widgets/WP_Menu.QuestIndex` 6 (`self.Menu`))
    (goto _label_5)))

(fn `AddItem`
  (params (ItemName :type Text) (ItemDescription :type Text) (ItemImage :type "SlateBrush Structure"))
  (`/Game/Widgets/InventoryWidgets/BPC_Inventory.AddItem` (`self.BPC_Inventory`) ItemName ItemDescription)
  (`/Game/Widgets/WP_Menu.Add Item` (`self.Menu`) ItemImage (`KismetArrayLibrary.Array_LastIndex` (`/Game/Widgets/InventoryWidgets/BPC_Inventory.ItemNameArray` (`self.BPC_Inventory`)))))

(fn `SwapItem`
  (params (ItemID :type Integer))
  (bind _bpc_inventory (`self.BPC_Inventory`))
  (bind _output (`|GetArrayItem` (`/Game/Widgets/InventoryWidgets/BPC_Inventory.ItemNameArray` _bpc_inventory) ItemID))
  ;[1 1 1] Swap Item (Keagon)
  (`KismetSystemLibrary.PrintText` _output)
  (`/Game/Widgets/WP_Menu.Swap Item` (`self.Menu`) _output (`|GetArrayItem` (`/Game/Widgets/InventoryWidgets/BPC_Inventory.ItemDescriptionArray` _bpc_inventory) ItemID)))

(fn `UserConstructionScript`)