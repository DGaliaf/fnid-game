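; BP_IntroPt2 is an overlap trigger actor that starts the second part of an intro by playing an assigned level sequence.
; On any actor overlap it casts the game instance to BP_GameVariables and checks the IntroWalk flag.
; When the flag is set it plays LevelSequenceToPlay, destroys itself so it fires once, and prints a debug string.
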(event `self.ReceiveActorBeginOverlap`
  (params (OtherActor :type "Actor Object Reference"))
  (bind _asbp_game_variables (cast `/Game/Blueprints/BP_GameVariables` (`GameplayStatics.GetGameInstance`))
    (:`then`
      (if (`/Game/Blueprints/BP_GameVariables.Intro Walk` _asbp_game_variables)
        (`MovieSceneSequencePlayer.Play` (`LevelSequenceActor.SequencePlayer` (`self.Level Sequence to Play`)))
        (`self.K2_DestroyActor`)
        (`KismetSystemLibrary.PrintString` "AHHHHHH")))
    (:`CastFailed`
      (`KismetSystemLibrary.PrintString` "Cast Failed"))))

(fn `UserConstructionScript`
  (`parent.UserConstructionScript`))