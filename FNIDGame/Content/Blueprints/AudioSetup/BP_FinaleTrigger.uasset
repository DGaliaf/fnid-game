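; BP_FinaleTrigger is an overlap trigger that starts the game's ending and sends the player to the credits.
; On any actor overlap, it checks the circuit, wires and buttons completion flags in the BP_GameVariables game instance.
; When all three are set, it plays a level sequence and disables the player character's WASD movement.
; After a fixed delay, rather than a sequence-finished callback, it removes all widgets and opens the credits level.
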(event `self.ReceiveActorBeginOverlap`
  (params (OtherActor :type "Actor Object Reference"))
  (bind _asbp_game_variables (cast `/Game/Blueprints/BP_GameVariables` (`GameplayStatics.GetGameInstance`))
    (:`then`
      (if (and (`/Game/Blueprints/BP_GameVariables.CircuitComplete` _asbp_game_variables) (`/Game/Blueprints/BP_GameVariables.WiresComplete` _asbp_game_variables) (`/Game/Blueprints/BP_GameVariables.ButtonsCompelte` _asbp_game_variables))
        (`MovieSceneSequencePlayer.Play` (`LevelSequenceActor.SequencePlayer` (`self.Level Sequence to Play`)))
        (bind _asbp_player_character_final (cast `/Game/Blueprints/BP_PlayerCharacterFinal` (`GameplayStatics.GetPlayerCharacter` 0)))
        (set `/Game/Blueprints/BP_PlayerCharacterFinal.WASD Movement` false _asbp_player_character_final)
        (`KismetSystemLibrary.PrintString` "AHHHHHH")
        (`KismetSystemLibrary.Delay` 6.3)
        (`WidgetLayoutLibrary.RemoveAllWidgets`)
        (`GameplayStatics.OpenLevelBySoftObjectPtr` "/Game/Levels/Credits_Level.Credits_Level")))
    (:`CastFailed`
      (`KismetSystemLibrary.PrintString` "Cast Failed"))))

(fn `UserConstructionScript`
  (`parent.UserConstructionScript`))