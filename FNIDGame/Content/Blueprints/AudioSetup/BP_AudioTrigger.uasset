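; BP_AudioTrigger is a one-time trigger actor that plays an assigned level sequence when the player character overlaps it.
; It then casts the game instance to BP_GameVariables, waits for Duration, sets the IntroWalk flag and destroys itself.
; A failed cast only prints a debug message, leaving the trigger in the level after the sequence has started.
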(event `self.ReceiveActorBeginOverlap`
  (params (OtherActor :type "Actor Object Reference"))
  (if (== OtherActor (`GameplayStatics.GetPlayerCharacter` 0))
    (`MovieSceneSequencePlayer.Play` (`LevelSequenceActor.SequencePlayer` (`self.Level Sequence to Play`)))
    (bind _asbp_game_variables (cast `/Game/Blueprints/BP_GameVariables` (`GameplayStatics.GetGameInstance`))
      (:`then`
        (`KismetSystemLibrary.Delay` (`self.Duration`))
        (set `/Game/Blueprints/BP_GameVariables.Intro Walk` true _asbp_game_variables)
        (`KismetSystemLibrary.PrintString` "Walk Set")
        (`self.K2_DestroyActor`))
      (:`CastFailed`
        (`KismetSystemLibrary.PrintString` "Cast Failed")))))

(fn `UserConstructionScript`)