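; BP_AudioTriggerPressure is a one-shot trigger actor that fires when the player character overlaps it.
; On overlap it plays its assigned level sequence and adds a W_InteractionHandles widget to the viewport.
; After a short delay it looks up top-level widgets of that class rather than reusing the created reference, removes them, and destroys itself.
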(event `self.ReceiveActorBeginOverlap`
  (params (OtherActor :type "Actor Object Reference"))
  (if (== OtherActor (`GameplayStatics.GetPlayerCharacter` 0))
    (`MovieSceneSequencePlayer.Play` (`LevelSequenceActor.SequencePlayer` (`self.Level Sequence to Play`)))
    (bind _returnvalue (`|CreateWidget` "/Game/Widgets/W_InteractionHandles.W_InteractionHandles_C"))
    (`UserWidget.AddToViewport` _returnvalue 0)
    (`KismetSystemLibrary.Delay` 5.0)
    (bind _foundwidgets (`WidgetBlueprintLibrary.GetAllWidgetsOfClass` "/Game/Widgets/W_InteractionHandles.W_InteractionHandles_C"))
    (`Widget.RemoveFromParent` _foundwidgets)
    (`self.K2_DestroyActor`)))

(fn `UserConstructionScript`)