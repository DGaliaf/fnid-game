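; BP_Door is a sliding double door meant to be gated by the keycard state stored in BP_GameVariables.
; InteractwithObject is empty, and the keycard branch that plays pass/fail sequences, shows W_NoAccess or slides DoorR and DoorL open is disconnected.
; The live logic runs three seconds after DoorCollision end overlap: if DoorOpen is set, a timeline slides both panels back by accumulating relative X offsets.
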(event `self.InteractWithObject`
  ;[1 1 1] Проверка моно ли открыть дверь
)

(event `self.Door Collision.OnComponentEndOverlap`
  (params (OverlappedComponent :type "PrimitiveComponent Object Reference") (OtherActor :type "Actor Object Reference") (OtherComp :type "PrimitiveComponent Object Reference") (OtherBodyIndex :type Integer))
  (bind (_relativelocation_x _relativelocation_y _relativelocation_z) (`KismetMathLibrary.BreakVector` (`SceneComponent.RelativeLocation` (`self.DoorR`))))
  (bind (_relativelocation_x_2 _relativelocation_y_2 _relativelocation_z_2) (`KismetMathLibrary.BreakVector` (`SceneComponent.RelativeLocation` (`self.DoorL`))))
  (`KismetSystemLibrary.Delay` 3.0)
  (cast `Character` (`GameplayStatics.GetPlayerCharacter` 0))
  (if (`self.DoorOpen`)
    (bind (_direction _newtrack_0) (`Timeline|Timeline_0` :!via `PlayFromStart`)
      (:`Update`
        (`SceneComponent.K2_SetRelativeLocation` (`self.DoorR`) (`KismetMathLibrary.MakeVector` (+ (* _newtrack_0 -1.0) _relativelocation_x) _relativelocation_y _relativelocation_z) false false)
        (`SceneComponent.K2_SetRelativeLocation` (`self.DoorL`) (`KismetMathLibrary.MakeVector` (+ (* _newtrack_0 1.0) _relativelocation_x_2) _relativelocation_y_2 _relativelocation_z_2) false false)
        (set `self.DoorOpen` false)))))

(fn `UserConstructionScript`
  (`parent.UserConstructionScript`))