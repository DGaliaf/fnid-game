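; A rotatable dial in a circuit puzzle that turns in quarter steps when interacted with, until the circuit is complete.
; Each dial writes its step to a shared rotation array in BP_GameVariables, then nested comparisons test that array against two accepted routes.
; Solving it sets CircuitComplete, plays a sound and restores walking.
; If the button and wire puzzles are also complete, music fades and a level sequence plays with WASD movement temporarily disabled.
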(event `self.InteractWithObject`
  (bind _returnvalue (`GameplayStatics.GetGameInstance`))
  (bind _rotatecount (`self.RotateCount`))
  (bind _asbp_game_variables (cast `/Game/Blueprints/BP_GameVariables` _returnvalue))
  (if (not (`/Game/Blueprints/BP_GameVariables.CircuitComplete` _asbp_game_variables))
    (`SceneComponent.K2_SetRelativeRotation` (`self.Dial`) (`KismetMathLibrary.MakeRotator` 0.0 (* _rotatecount -90.0)) false false)
    (bind _asbp_game_variables_2 (cast `/Game/Blueprints/BP_GameVariables` _returnvalue)
      (:`then`
        (bind _output_get (set `self.RotateCount` (mod (+ _rotatecount 1) 4)))
        (bind _dial_rotations (`/Game/Blueprints/BP_GameVariables.Dial Rotations` _asbp_game_variables_2))
        (`KismetArrayLibrary.Array_Set` _dial_rotations (`self.DialCount`) _output_get)
        (`/Engine/EditorBlueprintResources/StandardMacros.CompareInt` (`|GetArrayItem` _dial_rotations) 3
          (:`==`
            (`/Engine/EditorBlueprintResources/StandardMacros.CompareInt` (`|GetArrayItem` _dial_rotations 1) 1
              (:`==`
                (`/Engine/EditorBlueprintResources/StandardMacros.CompareInt` (`|GetArrayItem` _dial_rotations 5) 2
                  (:`>`
                    (`/Engine/EditorBlueprintResources/StandardMacros.CompareInt` (`|GetArrayItem` _dial_rotations 5) 3 :!label _label
                      (:`==`
                        (`/Engine/EditorBlueprintResources/StandardMacros.CompareInt` (`|GetArrayItem` _dial_rotations 6) 1
                          (:`==`
                            (`/Engine/EditorBlueprintResources/StandardMacros.CompareInt` (`|GetArrayItem` _dial_rotations 10) 3
                              (:`==`
                                (`/Engine/EditorBlueprintResources/StandardMacros.CompareInt` (`|GetArrayItem` _dial_rotations 11) 1
                                  (:`==`
                                    (`/Engine/EditorBlueprintResources/StandardMacros.CompareInt` (`|GetArrayItem` _dial_rotations 15) 3
                                      (:`==`
                                        _)))))))))))
                  (:`==`
                    (`/Engine/EditorBlueprintResources/StandardMacros.CompareInt` (`|GetArrayItem` _dial_rotations 4)
                      (:`==`
                        (`/Engine/EditorBlueprintResources/StandardMacros.CompareInt` (`|GetArrayItem` _dial_rotations 8) 3
                          (:`==`
                            (`/Engine/EditorBlueprintResources/StandardMacros.CompareInt` (`|GetArrayItem` _dial_rotations 9) 1
                              (:`==`
                                (`/Engine/EditorBlueprintResources/StandardMacros.CompareInt` (`|GetArrayItem` _dial_rotations 13) 3
                                  (:`==`
                                    (`/Engine/EditorBlueprintResources/StandardMacros.CompareInt` (`|GetArrayItem` _dial_rotations 14) 2
                                      (:`==`
                                        (`/Engine/EditorBlueprintResources/StandardMacros.CompareInt` (`|GetArrayItem` _dial_rotations 10)
                                          (:`==`
                                            (`/Engine/EditorBlueprintResources/StandardMacros.CompareInt` (`|GetArrayItem` _dial_rotations 11) 1
                                              (:`==`
                                                (`/Engine/EditorBlueprintResources/StandardMacros.CompareInt` (`|GetArrayItem` _dial_rotations 15) 3
                                                  (:`==`
                                                    _)))))))))))))))))
                  (:`<`
                    (goto _label)))
                (bind _asbp_game_variables_3 (cast `/Game/Blueprints/BP_GameVariables` (`GameplayStatics.GetGameInstance`)))
                (bind _output_get_2 (set `/Game/Blueprints/BP_GameVariables.CircuitComplete` true _asbp_game_variables_3))
                (`KismetSystemLibrary.PrintString` (`KismetStringLibrary.Conv_BoolToString` _output_get_2))
                (`GameplayStatics.PlaySound2D` "/Game/Audio/Ambient/Sounds/Accepting_Harmony.Accepting_Harmony" 1.0 1.0 0.0 null null)
                (`CharacterMovementComponent.SetMovementMode` (`Character.CharacterMovement` (`GameplayStatics.GetPlayerCharacter` 0)) "MOVE_Walking" 0)
                (bind _asbp_game_variables_4 (cast `/Game/Blueprints/BP_GameVariables` (`GameplayStatics.GetGameInstance`)))
                (if (and (`/Game/Blueprints/BP_GameVariables.ButtonsCompelte` _asbp_game_variables_4) (`/Game/Blueprints/BP_GameVariables.CircuitComplete` _asbp_game_variables_4) (`/Game/Blueprints/BP_GameVariables.WiresComplete` _asbp_game_variables_4))
                  (bind _asbp_screen_changer (cast `/Game/Blueprints/BP_ScreenChanger` (`self.Screen Changer`)))
                  (`AudioComponent.FadeOut` (`/Game/Blueprints/BP_ScreenChanger.MusicRef` _asbp_screen_changer) 5.0 0.0 "Linear")
                  (bind _asbp_player_character_ace (cast `/Game/Blueprints/BP_PlayerCharacterACE` (`GameplayStatics.GetPlayerCharacter` 0)))
                  (set `/Game/Blueprints/BP_PlayerCharacterACE.WASD Movement` false _asbp_player_character_ace)
                  (`MovieSceneSequencePlayer.Play` (`LevelSequenceActor.SequencePlayer` (`self.Level Sequencer`)))
                  (`KismetSystemLibrary.Delay` 13.5)
                  (set `/Game/Blueprints/BP_PlayerCharacterACE.WASD Movement` true _asbp_player_character_ace)))))))
      (:`CastFailed`
        (`KismetSystemLibrary.PrintString` "Cast Failed")))))

(fn `UserConstructionScript`
  (`parent.UserConstructionScript`))