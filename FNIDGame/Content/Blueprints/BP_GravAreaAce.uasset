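; BP_GravAreaAce is a trigger volume that disrupts player gravity until the button, circuit and wire tasks in BP_GameVariables are all complete.
; On overlap it halves the player's velocity and turns off their Gravity flag.
; Volumes marked GeneratorRoomBox also set GeneratorRoomPlayer and pulse gravity through a delayed loop that repeats while the overlap lasts.
; Leaving the box restores gravity and clears the generator-room flag.
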(event `self.Box.OnComponentBeginOverlap`
  (params (OverlappedComponent :type "PrimitiveComponent Object Reference") (OtherActor :type "Actor Object Reference") (OtherComp :type "PrimitiveComponent Object Reference") (OtherBodyIndex :type Integer) (bFromSweep :type Boolean) (SweepResult :type "HitResult Structure (by ref)"))
  (bind _asbp_player_character_ace (cast `/Game/Blueprints/BP_PlayerCharacterFinal` OtherActor))
  (if (`self.IsOverlappingActor` _asbp_player_character_ace) :!label _label
    (bind _asbp_game_variables (cast `/Game/Blueprints/BP_GameVariables` (`GameplayStatics.GetGameInstance`)))
    (if (not (and (`/Game/Blueprints/BP_GameVariables.ButtonsCompelte` _asbp_game_variables) (`/Game/Blueprints/BP_GameVariables.CircuitComplete` _asbp_game_variables) (`/Game/Blueprints/BP_GameVariables.WiresComplete` _asbp_game_variables)))
      (bind _charactermovement (`Character.CharacterMovement` _asbp_player_character_ace))
      (set `MovementComponent.Velocity` (/ (`MovementComponent.Velocity` _charactermovement) 2) _charactermovement)
      (set `/Game/Blueprints/BP_PlayerCharacterFinal.gravity` false _asbp_player_character_ace)
      (if (`self.GeneratorRoom?Box`)
        (set `/Game/Blueprints/BP_PlayerCharacterFinal.GeneratorRoom?Player` true _asbp_player_character_ace)
        (`KismetSystemLibrary.Delay` (`self.DelayDuration`))
        (set `/Game/Blueprints/BP_PlayerCharacterFinal.gravity` true _asbp_player_character_ace)
        (`KismetSystemLibrary.Delay` (`self.DelayDuration`))
        (`KismetSystemLibrary.PrintString` "Hello")
        (goto _label)
        (else
          (set `/Game/Blueprints/BP_PlayerCharacterFinal.GeneratorRoom?Player` false _asbp_player_character_ace))))))

(event `self.Box.OnComponentEndOverlap`
  (params (OverlappedComponent :type "PrimitiveComponent Object Reference") (OtherActor :type "Actor Object Reference") (OtherComp :type "PrimitiveComponent Object Reference") (OtherBodyIndex :type Integer))
  (bind _asbp_player_character_ace (cast `/Game/Blueprints/BP_PlayerCharacterFinal` OtherActor))
  (set `/Game/Blueprints/BP_PlayerCharacterFinal.gravity` true _asbp_player_character_ace)
  (set `/Game/Blueprints/BP_PlayerCharacterFinal.GeneratorRoom?Player` false _asbp_player_character_ace)
  (`KismetSystemLibrary.PrintString` "Hello"))

(fn `UserConstructionScript`)