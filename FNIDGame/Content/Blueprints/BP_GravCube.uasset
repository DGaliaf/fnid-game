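; BP_GravCube is a physics cube that follows the player character's Gravity state, checked every Tick.
; While gravity is off, it floats via small upward and random sideways impulses, and sets Slam from the player's GeneratorRoomPlayer flag.
; While gravity is on, it re-enables cube gravity and, if Slam is set, applies strong downward, sideways and spin impulses every frame.
; NegativeArray supplies random multipliers for the randomized impulses.
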(event `self.ReceiveTick`
  (params (DeltaSeconds :type "Float (single-precision)"))
  (bind _returnvalue (* (`KismetMathLibrary.RandomFloatInRange` 9000.0 10000.0) (`KismetArrayLibrary.Array_Random` (`self.negativeArray`))))
  (bind _returnvalue_2 (* (`KismetMathLibrary.RandomFloatInRange` 50.0 100.0) (`KismetArrayLibrary.Array_Random` (`self.negativeArray`))))
  (bind _returnvalue_3 (* (`KismetMathLibrary.RandomFloatInRange` 1999.0 2000.0) (`KismetArrayLibrary.Array_Random` (`self.negativeArray`))))
  (bind _asbp_player_character_final (cast `/Game/Blueprints/BP_PlayerCharacterFinal` (`GameplayStatics.GetPlayerPawn` 0)))
  (if (`/Game/Blueprints/BP_PlayerCharacterFinal.gravity` _asbp_player_character_final)
    (if (`self.Slam?`)
      (`PrimitiveComponent.AddImpulse` (`self.Cube`) (`KismetMathLibrary.MakeVector` _returnvalue_3 _returnvalue_3 -20000.0) "None" false)
      (`PrimitiveComponent.AddAngularImpulseInDegrees` (`self.Cube`) (`KismetMathLibrary.MakeVector` _returnvalue _returnvalue _returnvalue) "None" false))
    (`PrimitiveComponent.SetEnableGravity` (`self.Cube`) true)
    (else
      (if (`/Game/Blueprints/BP_PlayerCharacterFinal.GeneratorRoom?Player` _asbp_player_character_final)
        (set `self.Slam?` true)
        (else
          (set `self.Slam?` false)))
      (`PrimitiveComponent.SetEnableGravity` (`self.Cube`) false)
      (`PrimitiveComponent.AddImpulse` (`self.Cube`) (0.0 0.0 75.0) "None" false)
      (`PrimitiveComponent.AddImpulse` (`self.Cube`) (`KismetMathLibrary.MakeVector` _returnvalue_2 _returnvalue_2) "None" false))))

(fn `UserConstructionScript`)